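; MainPlayer is the player character, turning input actions into movement, mouse look, jumping, crouch toggling and interaction.
; It pushes movement axes and jump and crouch states into the PlayerAnimation instance on its skeletal mesh.
; Crouch start and end events adjust the mesh's relative height from the half-height adjustment.
; Interact scans all BPI_Interactable actors and sends InteractMessage to every one within InteractDistance.
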(event Input|EnhancedActionEvents|EnhancedInputActionInteract
  (params (ActionValue :type Boolean) (ElapsedSeconds :type Float%20%28double-precision%29) (TriggeredSeconds :type Float%20%28double-precision%29) (InputAction :type Input%20Action%20Object%20Reference :default "/Game/SceneComponents/Keybinds/Interact.Interact"))
  (bind _outactors (Actor|GetAllActorswithInterface "/Game/BPI_Interactable.BPI_Interactable_C"))
  (for _array_element _outactors
    (if (<= (Math|Vector|Distance(Vector) (Transformation|GetActorLocation _array_element) (Transformation|GetActorLocation)) (Variables|Default|GetInteractDistance))
      (Class|BPIInteractable|Interact(Message) _array_element))))

(event Input|EnhancedActionEvents|EnhancedInputActionMoving
  (params (ActionValue :type Vector%202D%20Structure) (ElapsedSeconds :type Float%20%28double-precision%29) (TriggeredSeconds :type Float%20%28double-precision%29) (InputAction :type Input%20Action%20Object%20Reference :default "/Game/SceneComponents/Keybinds/Moving.Moving"))
  (bind (_x _y) (Math|Vector2D|BreakVector2D ActionValue))
  (Pawn|Input|AddMovementInput (* (Transformation|GetActorRightVector) _x) 1.0 false)
  (Pawn|Input|AddMovementInput (* _y (Transformation|GetActorForwardVector)) 1.0 false)
  (bind _asplayer_animation (Utilities|Casting|CastToPlayerAnimation (Components|SkeletalMesh|GetAnimInstance (Variables|Default|GetSkeletalMesh))))
  (Variables|/Game/Models/Player/AnimController/PlayerAnimation.PlayerAnimation_C|SetSpeedX _asplayer_animation _x)
  (Variables|/Game/Models/Player/AnimController/PlayerAnimation.PlayerAnimation_C|SetSpeedY _asplayer_animation _y))

(event Input|EnhancedActionEvents|EnhancedInputActionMouseLooking
  (params (ActionValue :type Vector%202D%20Structure) (ElapsedSeconds :type Float%20%28double-precision%29) (TriggeredSeconds :type Float%20%28double-precision%29) (InputAction :type Input%20Action%20Object%20Reference :default "/Game/SceneComponents/Keybinds/MouseLooking.MouseLooking"))
  (bind (_x _y) (Math|Vector2D|BreakVector2D ActionValue))
  (Pawn|Input|AddControllerYawInput _x)
  (Pawn|Input|AddControllerPitchInput _y))

(event Input|EnhancedActionEvents|EnhancedInputActionJump
  (params (ActionValue :type Boolean) (ElapsedSeconds :type Float%20%28double-precision%29) (TriggeredSeconds :type Float%20%28double-precision%29) (InputAction :type Input%20Action%20Object%20Reference :default "/Game/SceneComponents/Keybinds/Jump.Jump"))
  (Character|Jump)
  (bind _asplayer_animation (Utilities|Casting|CastToPlayerAnimation (Components|SkeletalMesh|GetAnimInstance (Variables|Default|GetSkeletalMesh))))
  (Variables|/Game/Models/Player/AnimController/PlayerAnimation.PlayerAnimation_C|SetJumping _asplayer_animation true))

(event Input|EnhancedActionEvents|EnhancedInputActionCrouch
  (params (ActionValue :type Boolean) (ElapsedSeconds :type Float%20%28double-precision%29) (TriggeredSeconds :type Float%20%28double-precision%29) (InputAction :type Input%20Action%20Object%20Reference :default "/Game/SceneComponents/Keybinds/Crouch.Crouch"))
  (bind _charactermovement (Variables|Character|GetCharacterMovement))
  (bind _returnvalue (AI|Components|NavMovement|IsCrouching _charactermovement))
  (if _returnvalue
    (Character|UnCrouch)
    (else
      (Character|Crouch)))
  (CallFunction|SetCrouching (not _returnvalue)))

(event EventOnStartCrouch
  (params (HalfHeightAdjust :type Float%20%28single-precision%29) (ScaledHalfHeightAdjust :type Float%20%28single-precision%29))
  (bind _result (Math|Float|NegateFloat ScaledHalfHeightAdjust)
    (:%20%20
      (Transformation|SetRelativeLocation (Variables|Default|GetSkeletalMesh) (Math|Vector|MakeVector 0.0 0.0 _result) false false))))

(event EventOnEndCrouch
  (params (HalfHeightAdjust :type Float%20%28single-precision%29) (ScaledHalfHeightAdjust :type Float%20%28single-precision%29))
  (bind _result (Math|Float|NegateFloat ScaledHalfHeightAdjust)
    (:%20%20
      (Transformation|SetRelativeLocation (Variables|Default|GetSkeletalMesh) (Math|Vector|MakeVector 0.0 0.0 _result) false false))))

(event EventOnLanded
  (params (Hit :type Hit%20Result%20Structure%20%28by%20ref%29))
  (CallFunction|SetJumping false))

(fn ConstructionScript)

(fn SetJumping
  (params (Value :type Boolean))
  (bind _asplayer_animation (Utilities|Casting|CastToPlayerAnimation (Components|SkeletalMesh|GetAnimInstance (Variables|Default|GetSkeletalMesh))))
  (Variables|/Game/Models/Player/AnimController/PlayerAnimation.PlayerAnimation_C|SetJumping _asplayer_animation Value))

(fn SetCrouching
  (params (Value :type Boolean))
  (bind _asplayer_animation (Utilities|Casting|CastToPlayerAnimation (Components|SkeletalMesh|GetAnimInstance (Variables|Default|GetSkeletalMesh))))
  (Variables|/Game/Models/Player/AnimController/PlayerAnimation.PlayerAnimation_C|SetCrouch _asplayer_animation Value))