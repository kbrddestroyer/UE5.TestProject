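; BP_NPC is an interactable NPC actor that turns with the player's position and shows a text label within interaction range.
; The construction script caches the first MainPlayer found.
; Tick sets yaw along the player-to-NPC direction and shows the TextRender within the player's InteractDistance.
; Interact toggles the Interacted flag on the mesh's BP_NPCAnim instance, leaving the response to the animation blueprint.
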(event EventBeginPlay)

(event Collision|EventActorBeginOverlap
  (params (OtherActor :type Actor%20Object%20Reference)))

(event EventTick
  (params (DeltaSeconds :type Float%20%28single-precision%29))
  (bind _returnvalue (Transformation|GetActorLocation))
  (bind _player (Variables|Default|GetPlayer))
  (bind _returnvalue_2 (Transformation|GetActorLocation _player))
  (Transformation|SetActorRotation (Math|Rotator|MakeRotator 0.0 0.0 (.Yaw (Math|Rotator|BreakRotator (Math|Rotator|FindLookatRotation _returnvalue_2 _returnvalue)))))
  (Rendering|SetVisibility (Variables|Default|GetTextRender) (<= (Math|Vector|Distance(Vector) _returnvalue_2 _returnvalue) (Variables|/Game/SceneComponents/Blueprint/MainPlayer.MainPlayer_C|GetInteractDistance (Variables|Default|GetPlayer))) false))

(event EventInteract
  (CallFunction|InteractFunc))

(fn ConstructionScript
  (bind _outactors (Actor|GetAllActorsOfClass "/Game/SceneComponents/Blueprint/MainPlayer.MainPlayer_C"))
  (Variables|Default|SetPlayer (Utilities|Array|Get(acopy) _outactors)))

(fn InteractFunc
  (bind _asbp_npcanim (Utilities|Casting|CastToBP_NPCAnim (Components|SkeletalMesh|GetAnimInstance (Variables|Default|GetSkeletalMesh))))
  (Variables|/Game/Animation/BP_NPCAnim.BP_NPCAnim_C|SetInteracted _asbp_npcanim (not (Variables|/Game/Animation/BP_NPCAnim.BP_NPCAnim_C|GetInteracted _asbp_npcanim))))